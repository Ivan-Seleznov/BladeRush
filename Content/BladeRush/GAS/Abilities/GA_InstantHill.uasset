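; Gameplay ability for an instant "Hill", apparently a syringe-style heal, that finishes as soon as it activates.
; Activation applies the Hill and ability-blocking effects to the owner, plays a syringe sound for the local player, commits the cooldown, then ends.
; CanActivate passes only when two float attributes read from the avatar differ, likely current versus maximum health.
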(event Ability|EventActivateAbility
  (Utilities|FlowControl|Sequence
    (:then_0
      (Ability|ApplyGameplayEffectToOwner (Variables|Default|GetHillGameplayEffect))
      (Ability|ApplyGameplayEffectToOwner (Variables|Default|GetBlockAbilitiesGameplayEffect)))
    (:then_1
      (Pawn|IsLocallyControlled
        (:True
          (Audio|PlaySound2D "/Game/Assets/Sounds/S_Syringe.S_Syringe" 1.0 1.0 0.0 0 0))))
    (:then_2
      (Ability|CommitAbilityCooldown false))
    (:then_3
      (Ability|EndAbility))))

(event Ability|EventOnEndAbility
  (params (bWasCancelled :type Boolean)))

(fn K2CanActivateAbility
  (params (ActorInfo :type Gameplay%20Ability%20Actor%20Info%20Structure) (Handle :type Gameplay%20Ability%20Spec%20Handle%20Structure))
  (return "" (not (Math|Float|NearlyEqual(Float) (.ReturnValue (Ability|Attribute|GetFloatAttribute (.avataractor ActorInfo) "(AttributeName=\"HitPoints\",Attribute=/Script/BladeRush.AttributeHitPoints:HitPoints,AttributeOwner=/Script/CoreUObject.Class'\"/Script/BladeRush.AttributeHitPoints\"')")) (.ReturnValue (Ability|Attribute|GetFloatAttribute (.avataractor ActorInfo) "(AttributeName=\"MaxHitPoints\",Attribute=/Script/BladeRush.AttributeHitPoints:MaxHitPoints,AttributeOwner=/Script/CoreUObject.Class'\"/Script/BladeRush.AttributeHitPoints\"')")) 1e-06))))