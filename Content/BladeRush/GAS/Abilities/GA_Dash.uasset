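; GA_Dash is a Gameplay Ability that drives the local player's dash feedback.
; On activation, for locally controlled players only, it prints the camera FOV, plays a 2D sound, and pushes a new BP_CameraMode_Dash object onto the BladeRush camera manager.
; On ability end it tells that camera mode object to exit, again only for the local player.
; The graph contains no movement logic and never calls EndAbility itself.
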(event Ability|EventActivateAbility
  (Pawn|IsLocallyControlled
    (:True
      (bind _asblade_rush_camera_manager (Utilities|Casting|CastToBladeRushCameraManager (Variables|/Script/Engine.PlayerController|GetPlayerCameraManager (.playercontroller (Ability|GetActorInfo)))))
      (Development|PrintString (Utilities|String|ToString(Float) (Camera|GetFOVAngle _asblade_rush_camera_manager)))
      (Audio|PlaySound2D (Variables|Default|GetSound) 1.0 1.0 0.0 0 0 false)
      (bind _asblade_rush_camera_manager_2 (Utilities|Casting|CastToBladeRushCameraManager (Variables|/Script/Engine.PlayerController|GetPlayerCameraManager (.playercontroller (Ability|GetActorInfo)))))
      (bind _returnvalue (Game|ConstructObjectfromClass "/Game/BladeRush/Camera/CameraModes/BP_CameraMode_Dash.BP_CameraMode_Dash_C"))
      (bind _output_get (Variables|Default|SetCameraModeObject _returnvalue))
      (Class|BladeRushCameraManager|SetCameraModeObject _asblade_rush_camera_manager_2 _output_get true))))

(event Ability|EventOnEndAbility
  (params (bWasCancelled :type Boolean))
  (Pawn|IsLocallyControlled
    (:True
      (Class|CameraMode|ExitCameraMode (Variables|Default|GetCameraModeObject)))))