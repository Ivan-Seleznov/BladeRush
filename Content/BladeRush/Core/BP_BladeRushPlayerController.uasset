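; Player controller for BladeRush that toggles a return-to-main-menu widget with the Escape key.
; A FlipFlop alternates between creating the widget in game-and-UI input with a visible cursor, and removing it to restore game-only input.
; Generic CreateWidget and DestroyWidget helpers handle viewport, input mode and cursor changes.
; On possession it sets game-only input and hides the cursor, a step marked for later removal.
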(event Custom|SetInputModeGameOnly
  ;[1 1 1] remove later
  (Input|SetInputModeGameOnly self false)
  (Variables|Default|SetbShowMouseCursor false))

(event EventBeginPlay)

(event EventTick
  (params (DeltaSeconds :type Float%20%28single-precision%29)))

(event EventPossess
  (params (PossessedPawn :type Pawn%20Object%20Reference))
  ;[1 1 1] remove later
  (CallFunction|SetInputModeGameOnly))

(event Input|KeyboardEvents|Escape
  (params (Key :type Key%20Structure :default "None"))
  (:Pressed
    (Utilities|FlowControl|FlipFlop
      (:A
        (bind _createdwidget (CallFunction|CreateWidget true "/Game/BladeRush/UI/MainMenu/WBP_ReturnToMainMenu.WBP_ReturnToMainMenu_C"))
        (Variables|Default|SetRerturnToMainMenuWidget _createdwidget))
      (:B
        (CallFunction|DestroyWidget (Variables|Default|GetRerturnToMainMenuWidget) true)))))

(fn ConstructionScript)

(fn CreateWidget
  (params (AddToViewPort :type Boolean) (WidgetClass :type User%20Widget%20Class%20Reference))
  (bind _returnvalue (UserInterface|CreateWidget WidgetClass self))
  (if AddToViewPort
    (UserInterface|Viewport|AddtoViewport _returnvalue 0))
  (Input|SetInputModeGameandUI self _returnvalue "DoNotLock" false false)
  (Variables|Default|SetbShowMouseCursor true)
  (return _returnvalue))

(fn DestroyWidget
  (params (InWidget :type User%20Widget%20Object%20Reference) (SetInputGameOnly :type Boolean))
  (Widget|RemovefromParent InWidget)
  (if SetInputGameOnly
    (Input|SetInputModeGameOnly self false)
    (Variables|Default|SetbShowMouseCursor false)))