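; GA_SpeedBoost is a Gameplay Ability that temporarily raises the owning character's movement speed.
; On activation, the authority sets the max speed multiplier on ShooterMovementComponent and starts a one-shot timer for the boost duration, intended to end the ability.
; Ending the ability resets the multiplier to normal and only then commits the cooldown, without an authority check.
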(event Custom|SpeedBoostTimer
  (Ability|EndAbility))

(event Ability|EventActivateAbility
  (Ability|HasAuthority
    (:True
      (Variables|/Script/BladeRush.ShooterMovementComponent|SetMaxSpeedMultiplier (Variables|/Script/BladeRush.BaseCharacter|GetShooterMovementComponent (Class|GameplayAbilityBase|GetCharacterfromActorInfo)) (Variables|Default|GetMax%20Speed%20Multiplier))
      (Utilities|Time|SetTimerbyEvent (EventDispatchers|CreateEvent :!event Custom|SpeedBoostTimer) (Variables|Default|GetSpeedBoostTime)))))

(event Ability|EventOnEndAbility
  (params (bWasCancelled :type Boolean))
  (Variables|/Script/BladeRush.ShooterMovementComponent|SetMaxSpeedMultiplier (Variables|/Script/BladeRush.BaseCharacter|GetShooterMovementComponent (Class|GameplayAbilityBase|GetCharacterfromActorInfo)) 1.0)
  (Ability|CommitAbilityCooldown false))