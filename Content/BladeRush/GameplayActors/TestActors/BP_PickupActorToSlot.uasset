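; BP_PickupActorToSlot is a test pickup that gives an overlapping BaseCharacter an item in a specific quick bar slot.
; On authority, overlap adds ItemDef with StackCount to the controller's InventoryManagerComponent.
; The new item instance goes to the character's QuickBarComponent at SlotIndex as the active slot, then FinishPickup runs with a debug print.
; The construction script displays SlotIndex on SlotText.
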(event Collision|EventActorBeginOverlap
  (params (OtherActor :type Actor%20Object%20Reference))
  (Networking|SwitchHasAuthority
    (:Authority
      (bind _asbase_character (Utilities|Casting|CastToBaseCharacter OtherActor))
      (Utilities|IsValid (Actor|GetComponentbyClass (Pawn|GetController _asbase_character) "/Script/BladeRush.InventoryManagerComponent")
        (:Is%20Valid
          (bind _returnvalue (Class|InventoryManagerComponent|AddItemDefinition (Actor|GetComponentbyClass (Pawn|GetController _asbase_character) "/Script/BladeRush.InventoryManagerComponent") (Variables|Default|GetItem%20Def) (Variables|Default|GetStack%20Count)))
          (Utilities|IsValid _returnvalue
            (:Is%20Valid
              (Utilities|IsValid (Actor|GetComponentbyClass _asbase_character "/Script/BladeRush.QuickBarComponent")
                (:Is%20Valid
                  (Class|QuickBarComponent|TryAddItemtoSlot (Actor|GetComponentbyClass _asbase_character "/Script/BladeRush.QuickBarComponent") _returnvalue (Variables|Default|GetSlotIndex) true)
                  (Development|PrintString "Item Added To slot " true true "(R=0.299575,G=1.000000,B=0.504232,A=1.000000)")
                  (CallFunction|FinishPickup))))))
        (:Is%20Not%20Valid
          (Development|PrintString "Inventory Comp not found"))))))

(fn ConstructionScript
  (|CallParentFunction)
  (Class|Text3DComponent|SetText (Variables|Default|GetSlotText) (Utilities|Text|ToText(Integer) (Variables|Default|GetSlotIndex))))