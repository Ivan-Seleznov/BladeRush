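; Test pickup actor that gives an overlapping BaseCharacter an item and equips it.
; On the server, overlap adds the ItemDef stack to the controller's InventoryManagerComponent, then equips its EquippableItemFragment's equipment definition through the character's EquipmentManagerComponent.
; Only a successful equip can destroy the pickup, if configured; outcomes print as debug strings.
; Construction script applies mesh, scale, collision radius and 3D label from exposed settings.
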(event Collision|EventActorBeginOverlap
  (params (OtherActor :type Actor%20Object%20Reference))
  (Networking|SwitchHasAuthority
    (:Authority
      (bind _asbase_character (Utilities|Casting|CastToBaseCharacter OtherActor))
      (Utilities|IsValid (Actor|GetComponentbyClass (Pawn|GetController _asbase_character) "/Script/BladeRush.InventoryManagerComponent")
        (:Is%20Valid
          (bind _returnvalue (Class|InventoryManagerComponent|AddItemDefinition (Actor|GetComponentbyClass (Pawn|GetController _asbase_character) "/Script/BladeRush.InventoryManagerComponent") (Variables|Default|GetItem%20Def) (Variables|Default|GetStack%20Count)))
          (bind _returnvalue_2 (Class|InventoryItemInstance|FindFragmentbyClass _returnvalue "/Script/BladeRush.EquippableItemFragment"))
          (Utilities|IsValid (Actor|GetComponentbyClass _asbase_character "/Script/BladeRush.EquipmentManagerComponent")
            (:Is%20Valid
              (Utilities|IsValid _returnvalue_2
                (:Is%20Valid
                  (Class|EquipmentManagerComponent|EquipItem (Actor|GetComponentbyClass _asbase_character "/Script/BladeRush.EquipmentManagerComponent") (Variables|/Script/BladeRush.EquippableItemFragment|GetEquipmentDefinitionClass _returnvalue_2))
                  (Development|PrintString "Item added inventory and equipped" true true "(R=0.317172,G=1.000000,B=0.335987,A=1.000000)")
                  (CallFunction|FinishPickup))
                (:Is%20Not%20Valid
                  (Development|PrintString "Equipable item fragment not found"))))
            (:Is%20Not%20Valid
              (Development|PrintString "Equipm Comp not found"))))
        (:Is%20Not%20Valid
          (Development|PrintString "Inventory Comp not found"))))))

(fn ConstructionScript
  (bind _meshscale (Variables|Default|GetMeshScale))
  (Components|StaticMesh|SetStaticMesh (Variables|Default|GetStaticMesh) (Variables|Default|GetMesh))
  (Components|Sphere|SetSphereRadius (Variables|Default|GetSphere) (Variables|Default|GetSphereCollisionRadius) true)
  (Transformation|SetRelativeScale3D (Variables|Default|GetStaticMesh) (Math|Vector|MakeVector _meshscale _meshscale _meshscale))
  (Class|Text3DComponent|SetText (Variables|Default|GetText3D) (Utilities|GetClassDefaults (Variables|Default|GetItem%20Def))))

(fn FinishPickup
  (if (Variables|Default|GetDestroyAfterPickup)
    (Actor|DestroyActor)))