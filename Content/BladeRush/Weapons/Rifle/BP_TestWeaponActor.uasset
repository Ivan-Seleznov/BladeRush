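; Test weapon actor in the Rifle folder whose event graph is effectively inert.
; BeginPlay, HandleHit, Tick and OnExitADS are empty, and OnEnterADS only casts the owner to BaseCharacter.
; Disconnected nodes retain hit-marker logic that never runs: creating WBP_HitMarker for the locally controlled owner, and playing a 2D sound when a hit BaseCharacter still has health.
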(event EventBeginPlay)

(event EventTick
  (params (DeltaSeconds :type Float%20%28single-precision%29)))

(event EventOnEnterADS
  (params (WeaponInstance :type Weapon%20Item%20Instance%20Object%20Reference))
  (Utilities|Casting|CastToBaseCharacter (Components|GetOwner)))

(event EventHandleHit
  (params (Hit :type Hit%20Result%20Structure)))

(event EventOnExitADS
  (params (WeaponInstance :type Weapon%20Item%20Instance%20Object%20Reference)))

(fn ConstructionScript)