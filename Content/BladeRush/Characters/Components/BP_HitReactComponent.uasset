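; BP_HitReactComponent handles a character's reaction to being hit.
; OnHitReact applies a velocity-change impulse to the hit character along the hit direction and, if that character is locally controlled, adds a hit react widget to the viewport.
; A separate EnableRagdoll function disables movement, ignores capsule collision and turns on mesh physics, but is not called here.
; The hit animation node is disconnected, so it never plays.
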(event EventOnHitReact
  (params (HitResult :type Hit%20Result%20Structure%20%28by%20ref%29) (HitDirection :type Vector%20%28by%20ref%29 :default "0, 0, 0"))
  (bind _asbase_character (Utilities|Casting|CastToBaseCharacter (.HitActor (Collision|BreakHitResult HitResult))))
  (Physics|AddImpulse (Variables|/Script/Engine.Character|GetCharacterMovement _asbase_character) (* HitDirection (Variables|Default|GetImpulseStrength)) true)
  (if (Pawn|IsLocallyControlled _asbase_character)
    (bind _asplayer_controller (Utilities|Casting|CastToPlayerController (Pawn|GetController _asbase_character)))
    (bind _returnvalue (UserInterface|CreateWidget (Variables|Default|GetHitReactWidgetClass) _asplayer_controller))
    (UserInterface|Viewport|AddtoViewport _returnvalue 0)))

(fn EnableRagdoll
  (params (Character :type Base%20Character%20Object%20Reference))
  (bind _mesh (Variables|/Script/Engine.Character|GetMesh Character))
  (Pawn|Components|CharacterMovement|DisableMovement (Variables|/Script/BladeRush.BaseCharacter|GetShooterMovementComponent Character))
  (Collision|SetCollisionResponsetoAllChannels (Variables|/Script/Engine.Character|GetCapsuleComponent Character) "ECR_Ignore")
  (Collision|SetCollisionEnabled _mesh "QueryAndPhysics")
  (Physics|SetSimulatePhysics _mesh true))